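; BP_PressureSwitch is a pressure plate that switches on while an actor overlaps it and off when the overlap ends.
; Begin and end overlap send OnMessage or OffMessage to its Target reference and set the IsOn flag.
; The Cube mesh shifts down and back up to show the press, with a debug string printed on each change.
; Overlaps are not counted, so any single exit turns it off.
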(event EventBeginPlay)

(event EventTick
  (params (DeltaSeconds :type Float%20%28single-precision%29)))

(event Collision|EventActorBeginOverlap
  (params (OtherActor :type Actor%20Object%20Reference))
  (Class|BPIToggleSwitch|On(Message) (Variables|Default|GetTarget))
  (Variables|Default|SetIsOn true)
  (Development|PrintString "Switch On")
  (Transformation|AddLocalOffset (Variables|Default|GetCube) "0, 0,-4.800000" false false))

(event Collision|EventActorEndOverlap
  (params (OtherActor :type Actor%20Object%20Reference))
  (Class|BPIToggleSwitch|Off(Message) (Variables|Default|GetTarget))
  (Variables|Default|SetIsOn false)
  (Development|PrintString "Switch Off")
  (Transformation|AddLocalOffset (Variables|Default|GetCube) "0, 0,4.800000" false false))

(fn ConstructionScript)