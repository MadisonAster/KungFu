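; BP_ToggleSwitch is a switch actor that toggles on and off each time an actor begins overlapping it.
; A FlipFlop alternates between sending OnMessage and OffMessage to its Target, stores the state in IsOn and prints it.
; The construction script puts a dynamic material instance on the Cube in the off color, and each toggle updates its Color parameter to match.
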(event EventBeginPlay)

(event Collision|EventActorBeginOverlap
  (params (OtherActor :type Actor%20Object%20Reference))
  (bind _target (Variables|Default|GetTarget))
  (bind _materialinst (Variables|Default|GetMaterialInst))
  (bind _isa (Utilities|FlowControl|FlipFlop)
    (:A
      (Class|BPIonOffSwitch|On(Message) _target)
      (Rendering|Material|SetVectorParameterValue _materialinst "Color" (Variables|Default|GetOnColor) :!class /Script/Engine.MaterialInstanceDynamic))
    (:B
      (Class|BPIonOffSwitch|Off(Message) _target)
      (Rendering|Material|SetVectorParameterValue _materialinst "Color" (Variables|Default|GetOffColor) :!class /Script/Engine.MaterialInstanceDynamic)))
  (Variables|Default|SetIsOn _isa)
  (Development|PrintString (select _isa "Switch On" "Switch Off")))

(event EventTick
  (params (DeltaSeconds :type Float%20%28single-precision%29)))

(fn ConstructionScript
  (bind _returnvalue (Rendering|Material|CreateDynamicMaterialInstance (Variables|Default|GetMaterial) "None" :!class /Script/Engine.KismetMaterialLibrary))
  (bind _output_get (Variables|Default|SetMaterialInst _returnvalue))
  (Rendering|Material|SetMaterial (Variables|Default|GetCube) 0 _output_get)
  (Rendering|Material|SetVectorParameterValue _output_get "Color" (Variables|Default|GetOffColor) :!class /Script/Engine.MaterialInstanceDynamic))