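; BP_ModeSwitch is an overlap-triggered switch that cycles through modes and tells a Target which mode is active.
; Each actor overlap advances CurrentMode, wrapping around the ModeColors array, recolors the cube and calls SetModeMessage on Target.
; The construction script creates the cube's dynamic material instance and applies the initial color and mode, also sending the message to Target at that stage.
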(event EventBeginPlay)

(event Collision|EventActorBeginOverlap
  (params (OtherActor :type Actor%20Object%20Reference))
  (bind _output_get (Variables|Default|SetCurrentMode (Math|Integer|%(Integer) (+ (Variables|Default|GetCurrentMode) 1) (Utilities|Array|Length (Variables|Default|GetModeColors)))))
  (Rendering|Material|SetVectorParameterValue (Variables|Default|GetMaterialInst) "Color" (Utilities|Array|Get(acopy) (Variables|Default|GetModeColors) _output_get) :!class /Script/Engine.MaterialInstanceDynamic)
  (Class|BPIModeSwitch|SetMode(Message) (Variables|Default|GetTarget) (Variables|Default|GetCurrentMode)))

(event EventTick
  (params (DeltaSeconds :type Float%20%28single-precision%29)))

(fn ConstructionScript
  (bind _returnvalue (Rendering|Material|CreateDynamicMaterialInstance (Variables|Default|GetMaterial) "None" :!class /Script/Engine.KismetMaterialLibrary))
  (bind _output_get (Variables|Default|SetMaterialInst _returnvalue))
  (Rendering|Material|SetMaterial (Variables|Default|GetCube) 0 _output_get)
  (Rendering|Material|SetVectorParameterValue _output_get "Color" (Utilities|Array|Get(acopy) (Variables|Default|GetModeColors) (Variables|Default|GetCurrentMode)) :!class /Script/Engine.MaterialInstanceDynamic)
  (Class|BPIModeSwitch|SetMode(Message) (Variables|Default|GetTarget) (Variables|Default|GetCurrentMode)))