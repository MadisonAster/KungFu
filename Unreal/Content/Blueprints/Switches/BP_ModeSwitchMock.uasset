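; BP_ModeSwitchMock is a mock mode switch actor that shows its current mode as the color of a sphere.
; The construction script creates a dynamic material instance, applies it to the Sphere and tints it with the ModeColors entry for CurrentMode.
; The SetMode event stores a new mode index and updates the instance's Color parameter from that array.
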(event EventBeginPlay)

(event Collision|EventActorBeginOverlap
  (params (OtherActor :type Actor%20Object%20Reference)))

(event EventTick
  (params (DeltaSeconds :type Float%20%28single-precision%29)))

(event EventSetMode
  (params (ModeIndex :type Integer))
  (bind _output_get (Variables|Default|SetCurrentMode ModeIndex))
  (Rendering|Material|SetVectorParameterValue (Variables|Default|GetMaterialInst) "Color" (Utilities|Array|Get(acopy) (Variables|Default|GetModeColors) _output_get) :!class /Script/Engine.MaterialInstanceDynamic))

(fn ConstructionScript
  (bind _returnvalue (Rendering|Material|CreateDynamicMaterialInstance (Variables|Default|GetMaterial) "None" :!class /Script/Engine.KismetMaterialLibrary))
  (bind _output_get (Variables|Default|SetMaterialInst _returnvalue))
  (Rendering|Material|SetMaterial (Variables|Default|GetSphere) 0 _output_get)
  (Rendering|Material|SetVectorParameterValue _returnvalue "Color" (Utilities|Array|Get(acopy) (Variables|Default|GetModeColors) (Variables|Default|GetCurrentMode)) :!class /Script/Engine.MaterialInstanceDynamic))